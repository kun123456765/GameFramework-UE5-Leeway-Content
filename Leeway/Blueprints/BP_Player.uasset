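; Player character Blueprint that handles stance switching, attack input and physical pushes, with debug prints on hits and overlaps.
; Key presses run locally, then pass through server and all-client RPC events so remote copies replay them.
; Left mouse plays an attack montage, Q cycles stances by linking anim class layers and updating the movement component's layer tag, and the jog/run toggle is empty.
; Main-mesh overlaps shove other mesh components away with an impulse.
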(event OnComponentHit(MainSkeletalMesh)
  (params (HitComponent :type Primitive%20Component%20Object%20Reference) (OtherActor :type Actor%20Object%20Reference) (OtherComp :type Primitive%20Component%20Object%20Reference) (NormalImpulse :type Vector :default "0, 0, 0") (Hit :type Hit%20Result%20Structure%20%28by%20ref%29))
  (Development|PrintText "Hit"))

(event OnComponentBeginOverlap(MainSkeletalMesh)
  (params (OverlappedComponent :type Primitive%20Component%20Object%20Reference) (OtherActor :type Actor%20Object%20Reference) (OtherComp :type Primitive%20Component%20Object%20Reference) (OtherBodyIndex :type Integer) (bFromSweep :type Boolean) (SweepResult :type Hit%20Result%20Structure%20%28by%20ref%29))
  (Development|PrintText (Utilities|Text|ToText(Object) OtherActor))
  (bind _asmesh_component (Utilities|Casting|CastToMeshComponent OtherComp))
  (Physics|AddImpulse _asmesh_component (* (Math|Vector|Normalize (- (Transformation|GetActorLocation OtherActor) (Transformation|GetActorLocation self))) 3.5e+04) "None" false))

(event OnComponentHit(CapsuleComponent)
  (params (HitComponent :type Primitive%20Component%20Object%20Reference) (OtherActor :type Actor%20Object%20Reference) (OtherComp :type Primitive%20Component%20Object%20Reference) (NormalImpulse :type Vector :default "0, 0, 0") (Hit :type Hit%20Result%20Structure%20%28by%20ref%29))
  (Development|PrintText "11Hit"))

(event OnComponentBeginOverlap(CapsuleComponent)
  (params (OverlappedComponent :type Primitive%20Component%20Object%20Reference) (OtherActor :type Actor%20Object%20Reference) (OtherComp :type Primitive%20Component%20Object%20Reference) (OtherBodyIndex :type Integer) (bFromSweep :type Boolean) (SweepResult :type Hit%20Result%20Structure%20%28by%20ref%29))
  (Development|PrintText "22Overlap"))

(event Input|EnhancedActionEvents|EnhancedInputActionLW_IA_Move
  (params (ActionValue :type Vector%202D%20Structure) (ElapsedSeconds :type Float%20%28double-precision%29) (TriggeredSeconds :type Float%20%28double-precision%29) (InputAction :type Input%20Action%20Object%20Reference :default "/LeewayFreamwork/Input/Actions/LW_IA_Move.LW_IA_Move")))

(event EventBeginPlay
  (|CallParentFunction)
  (Utilities|FlowControl|Sequence
    (:then_0
      (CallFunction|SwitchStance)
      (Development|PrintText "Swith Stance"))))

(event Collision|EventActorBeginOverlap
  (params (OtherActor :type Actor%20Object%20Reference))
  (|CallParentFunction OtherActor) ; This node is disabled and will not be called.\nDrag off pins to build functionality.
)

(event EventTick
  (params (DeltaSeconds :type Float%20%28single-precision%29))
  (|CallParentFunction DeltaSeconds) ; This node is disabled and will not be called.\nDrag off pins to build functionality.
)

(event Input|MouseEvents|LeftMouseButton
  (params (Key :type Key%20Structure :default "None"))
  (:Pressed
    (CallFunction|KeyPressedonClient Key)))

(event Input|KeyboardEvents|AnyKey
  (params (Key :type Key%20Structure :default "None"))
  (:Pressed
    (CallFunction|KeyPressedonClient Key)))

(event Custom|KeyPressedOnClient
  (params (Key :type Key%20Structure :default "None"))
  (CallFunction|DoKeyPressed Key)
  (CallFunction|KeyPressedonServer Key))

(event Custom|RPC_S2A_KeyPressed
  (params (Key :type Key%20Structure :default "None"))
  (if (not (Pawn|IsLocallyControlled self))
    (CallFunction|DoKeyPressed Key)))

(event Custom|KeyPressedOnServer
  (params (Key :type Key%20Structure :default "None"))
  (CallFunction|RPCS2AKeyPressed Key))

(event Custom|DoKeyPressed
  (params (Key :type Key%20Structure :default "None"))
  (Utilities|FlowControl|Sequence
    (:then_0
      (if (== Key "LeftMouseButton")
        (Animation|Montage|PlayMontage (Variables|Default|GetMainSkeletalMesh) "/Game/Leeway/Arts/Animations/Boxing/Retargeted_XANDRA/KB_Attack.KB_Attack")))
    (:then_1
      (if (== Key "LeftShift")
        (CallFunction|SwitchJogRun)))
    (:then_2
      (if (== Key "LeftControl")
        _))
    (:then_3
      (if (== Key "Q")
        (CallFunction|SwitchStance)))))

(fn ConstructionScript
  (|CallParentFunction))

(fn SwitchJogRun)

(fn SwitchStance
  (bind _layerstagmap (LocalVariables|GetLayersTagMap))
  (bind _output_get (LocalVariables|SetNeedUnlink (>= (Variables|Default|GetStanceIndex) 0)))
  (if _output_get
    (Class|SkeletalMeshComponent|UnlinkAnimClassLayers (Variables|Default|GetMainSkeletalMesh) (Utilities|Array|Get(acopy) (LocalVariables|GetLayersClassMap) (Variables|Default|GetStanceIndex))))
  (bind _result (Math|Integer|IncrementInt (Variables|Default|GetStanceIndex))
    (:%20%20
      (Variables|Default|SetStanceIndex (Math|Integer|%(Integer) _result (Utilities|Array|Length _layerstagmap)))
      (bind _asbase_character_movement_component (Utilities|Casting|CastToBaseCharacterMovementComponent (Variables|Character|GetCharacterMovement)))
      (|SetBy-RefVar (.currentanimlayerstag (Variables|/Script/Leeway.BaseCharacterMovementComponent|GetAnimParams _asbase_character_movement_component)) (Utilities|Array|Get(acopy) _layerstagmap (Variables|Default|GetStanceIndex)))
      (Components|SkeletalMesh|AnimationBlueprintLinking|LinkAnimClassLayers (Variables|Default|GetMainSkeletalMesh) (Utilities|Array|Get(acopy) (LocalVariables|GetLayersClassMap) (Variables|Default|GetStanceIndex))))))

(fn PlayMontage)