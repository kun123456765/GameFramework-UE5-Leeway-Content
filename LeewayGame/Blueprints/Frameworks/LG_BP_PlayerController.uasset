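; Player controller Blueprint that lets the player cycle the controlled character's stance with the Q key.
; It extends the parent's DoKeyPressed handler, calling ChangeStance when Q arrives.
; ChangeStance advances a stored index, wraps it by the length of LayersTagMap0, and writes that entry to the controlled BaseCharacter's Stance.
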(event EventBeginPlay)

(event EventTick
  (params (DeltaSeconds :type Float%20%28single-precision%29)))

(fn ConstructionScript
  (|CallParentFunction))

(fn DoKeyPressed
  (params (Key :type Key%20Structure))
  (|CallParentFunction Key)
  (LocalVariables|SetKeyLocalVar Key)
  (Utilities|FlowControl|Sequence
    (:then_0
      (if (== (LocalVariables|GetKeyLocalVar) "Q")
        (CallFunction|ChangeStance)))))

(fn ChangeStance
  (bind _layerstagmap_0 (Variables|Default|GetLayersTagMap_0))
  (bind _asbase_character (Utilities|Casting|CastToBaseCharacter (Pawn|GetControlledPawn)))
  (bind _result (Math|Integer|IncrementInt (Variables|Default|GetStanceIndex_0))
    (:%20%20
      (bind _output_get (Variables|Default|SetStanceIndex_0 (Math|Integer|%(Integer) _result (Utilities|Array|Length _layerstagmap_0))))
      (Variables|/Script/Leeway.BaseCharacter|SetStance _asbase_character (Utilities|Array|Get(acopy) _layerstagmap_0 _output_get)))))